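; PuncherBP is a character Blueprint for a melee puncher that damages the player and tracks its own health.
; The construction script snaps left and right punch collision components to middle-finger sockets on the mesh.
; The actor-wide Hit event applies fixed damage to player character 0, regardless of what was struck.
; AnyDamage subtracts incoming damage from Health while it remains above zero, with no death handling.
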(event `self.ReceiveBeginPlay`)

(event `self.ReceiveActorBeginOverlap`
  (params (OtherActor :type "Actor Object Reference")))

(event `self.ReceiveTick`
  (params (DeltaSeconds :type "Float (single-precision)")))

(event `self.ReceiveHit`
  (params (MyComp :type "PrimitiveComponent Object Reference") (Other :type "Actor Object Reference") (OtherComp :type "PrimitiveComponent Object Reference") (bSelfMoved :type Boolean) (HitLocation :type "Vector Structure") (HitNormal :type "Vector Structure") (NormalImpulse :type "Vector Structure") (Hit :type "HitResult Structure (by ref)"))
  (`GameplayStatics.ApplyDamage` (`GameplayStatics.GetPlayerCharacter` 0) 10.0))

(event `self.ReceiveAnyDamage`
  (params (Damage :type "Float (single-precision)") (DamageType :type "DamageType Object Reference") (InstigatedBy :type "Controller Object Reference") (DamageCauser :type "Actor Object Reference"))
  (bind _health (`self.Health`))
  (if (not (<= _health 0.0))
    (set `self.Health` (- _health Damage))))

(fn `UserConstructionScript`
  (bind _mesh (`self.Mesh`))
  (`SceneComponent.K2_AttachTo` (`self.PunchCollision_l`) _mesh "middle_02_l" "SnapToTarget" true)
  (`SceneComponent.K2_AttachTo` (`self.PunchCollision_r`) _mesh "middle_02_r" "SnapToTarget" true))